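; Player controller for a top-down camera that pans the player pawn over a procedural hex-grid map.
; BeginPlay finds the hex grid, stores its bounds and locks the mouse in Game and UI mode.
; Each Tick, MoveCamera combines directional input with smoothly ramped screen-edge mouse scrolling, scaled by a zoom-interpolated speed but not frame time.
; It clamps position to the grid size, with fixed height and rotation.
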(event EventBeginPlay
  ;[0.2389 0.6141 1] Set Input Mode
  (Variables|Default|SetCameraPawn (Game|Player|GetPlayerPawn 0))
  (bind _asbp_hex_grid_procedural (Utilities|Casting|CastToBP_HexGridProceduralClass "/Game/BP_HexGridProcedural.BP_HexGridProcedural_C"))
  (bind _returnvalue (Actor|GetActorOfClass _asbp_hex_grid_procedural))
  (bind _output_get (Variables|Default|SetMAP%20GRID _returnvalue))
  (Variables|Default|SetGrid%20Size%20X (* (.x (.BoxExtent (Collision|GetActorBounds _output_get false false))) 2.0))
  (Variables|Default|SetGridSizeY (* (.y (.BoxExtent (Collision|GetActorBounds _output_get false false))) 2.0))
  (Input|SetInputModeGameandUI self 0 "LockAlways" false false))

(event EventTick
  (params (DeltaSeconds :type Float%20%28single-precision%29))
  ;[1 0.09896 0.09896] Appeler la fonction MoveCamera
  (CallFunction|MoveCamera))

(event Input|ActionEvents|InputActionRight
  (params (Key :type Key%20Structure :default "None"))
  ;[0.3958 0.2148 0.08046] RIGHT
  (:Pressed
    (Variables|Default|SetCameraMovement (+ (Variables|Default|GetCameraMovement) "1.000000,0.000000,0.000000")))
  (:Released
    (Variables|Default|SetCameraMovement (- (Variables|Default|GetCameraMovement) "1.000000,0.000000,0.000000"))))

(event Input|ActionEvents|InputActionTop
  (params (Key :type Key%20Structure :default "None"))
  ;[0.4247 1 0.3851] TOP
  (:Pressed
    (Variables|Default|SetCameraMovement (- (Variables|Default|GetCameraMovement) "0.000000,1.000000,0.000000")))
  (:Released
    (Variables|Default|SetCameraMovement (+ (Variables|Default|GetCameraMovement) "0.000000,1.000000,0.000000"))))

(event Input|ActionEvents|InputActionBottom
  (params (Key :type Key%20Structure :default "None"))
  ;[0.01124 0.474 0.167] BOTTOM
  (:Pressed
    (Variables|Default|SetCameraMovement (+ (Variables|Default|GetCameraMovement) "0.000000,1.000000,0.000000")))
  (:Released
    (Variables|Default|SetCameraMovement (- (Variables|Default|GetCameraMovement) "0.000000,1.000000,0.000000"))))

(event Input|ActionEvents|InputActionLeft
  (params (Key :type Key%20Structure :default "None"))
  ;[1 0.5427 0.2033] LEFT
  (:Pressed
    (Variables|Default|SetCameraMovement (- (Variables|Default|GetCameraMovement) "1.000000,0.000000,0.000000")))
  (:Released
    (Variables|Default|SetCameraMovement (+ (Variables|Default|GetCameraMovement) "1.000000,0.000000,0.000000"))))

(fn ConstructionScript)

(fn MoveCamera
  (bind _returnvalue (Viewport|GetViewportSize))
  (bind _returnvalue_2 (Viewport|GetViewportSize))
  (bind _returnvalue_3 (Class|WidgetLayoutLibrary|GetMousePositiononViewport))
  (Variables|Default|SetMouseX (.x _returnvalue_3))
  (Variables|Default|SetMouseY (.y _returnvalue_3))
  (Transformation|SetActorLocationAndRotation (Variables|Default|GetCameraPawn) (Math|Vector|MakeVector (Math|Float|Clamp(Float) (.x (+ (Transformation|GetActorLocation (Variables|Default|GetCameraPawn)) (* (Utilities|Operators|Subtract (Math|Vector|Normalize (Variables|Default|GetCameraMovement)) (Math|Vector|MakeVector (- 1.0 (Math|Float|Clamp(Float) (Math|Float|NormalizetoRange (Variables|Default|GetMouseX) 0.0 (* (.x (Viewport|GetViewportSize)) 0.05)))) 0.0 0.0) (Math|Vector|MakeVector (* (Math|Float|Clamp(Float) (Math|Float|NormalizetoRange (Variables|Default|GetMouseX) (* (.x _returnvalue_2) 0.95) (.x _returnvalue_2))) -1.0) 0.0 0.0) (Math|Vector|MakeVector 0.0 (- 1.0 (Math|Float|Clamp(Float) (Math|Float|NormalizetoRange (Variables|Default|GetMouseY) 0.0 (* 0.05 (.y (Viewport|GetViewportSize)))))) 0.0) (Math|Vector|MakeVector 0.0 (* (Math|Float|Clamp(Float) (Math|Float|NormalizetoRange (Variables|Default|GetMouseY) (* 0.95 (.y _returnvalue)) (.y _returnvalue))) -1.0) 0.0)) (Math|Float|Lerp (Variables|Default|GetMinCameraSpeed) (Variables|Default|GetMaxCameraSpeed) (Variables|Default|GetCameraZoom))))) 0.0 (Variables|Default|GetGrid%20Size%20X)) (Math|Float|Clamp(Float) (.y (+ (Transformation|GetActorLocation (Variables|Default|GetCameraPawn)) (* (Utilities|Operators|Subtract (Math|Vector|Normalize (Variables|Default|GetCameraMovement)) (Math|Vector|MakeVector (- 1.0 (Math|Float|Clamp(Float) (Math|Float|NormalizetoRange (Variables|Default|GetMouseX) 0.0 (* (.x (Viewport|GetViewportSize)) 0.05)))) 0.0 0.0) (Math|Vector|MakeVector (* (Math|Float|Clamp(Float) (Math|Float|NormalizetoRange (Variables|Default|GetMouseX) (* (.x _returnvalue_2) 0.95) (.x _returnvalue_2))) -1.0) 0.0 0.0) (Math|Vector|MakeVector 0.0 (- 1.0 (Math|Float|Clamp(Float) (Math|Float|NormalizetoRange (Variables|Default|GetMouseY) 0.0 (* 0.05 (.y (Viewport|GetViewportSize)))))) 0.0) (Math|Vector|MakeVector 0.0 (* (Math|Float|Clamp(Float) (Math|Float|NormalizetoRange (Variables|Default|GetMouseY) (* 0.95 (.y _returnvalue)) (.y _returnvalue))) -1.0) 0.0)) (Math|Float|Lerp (Variables|Default|GetMinCameraSpeed) (Variables|Default|GetMaxCameraSpeed) (Variables|Default|GetCameraZoom))))) 0.0 (Variables|Default|GetGridSizeY)) 7e+02) (Math|Rotator|MakeRotator 0.0 0.0 -9e+01)))