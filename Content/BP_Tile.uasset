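; BP_Tile is a map tile that randomizes its elevation as either water level or raised ground.
; The construction script rolls the height, offsets the mesh vertically by it and passes it to the material's Elevation parameter for height-based coloring.
; At BeginPlay, a timeline starting at a random time drives the Color parameter's glow.
; Its red and green multipliers are randomized only in disconnected legacy nodes.
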(event EventBeginPlay
  (Components|Timeline|SetNewTime (Variables|Default|GetTimeline_0) (Math|Random|RandomFloatinRange 0.0 5.0))
  (bind _glow (Timeline|Timeline_0 Play)
    (:Update
      (Rendering|Material|SetVectorParameterValueonMaterials (Variables|Default|GetStaticMesh) "Color" (Math|Vector|MakeVector (* _glow (Variables|Default|GetRandom%20R)) (* _glow (Variables|Default|GetRandom%20G)) 1.0)))))

(fn ConstructionScript
  (bind _returnvalue (Math|Random|RandomFloatinRange -1.0 1.0))
  (bind _staticmesh (Variables|Default|GetStaticMesh))
  ;[1 1 1] Gestion de la hauteur d'une tuile
  (if (<= _returnvalue 0.0)
    (Variables|Default|SetHeight (Variables|Default|GetBaseWaterHeight))
    (else
      (Variables|Default|SetHeight (Math|Float|Clamp(Float) _returnvalue 0.1))))
  (Transformation|SetWorldLocation _staticmesh (+ (Transformation|GetWorldLocation _staticmesh) (Math|Vector|MakeVector 0.0 0.0 (+ (* (Variables|Default|GetHeight) (Variables|Default|GetStrenght)) (Variables|Default|GetOffset)))) false false)
  ;[1 1 1] Gestion de la couleur en fonction de la hauteur
  (Rendering|Material|SetScalarParameterValueonMaterials (Variables|Default|GetStaticMesh) "Elevation" (Variables|Default|GetHeight)))