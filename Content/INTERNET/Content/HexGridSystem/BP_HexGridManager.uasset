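; Hex grid manager that builds a staggered tile map in its Construction Script.
; Tiles are either instanced meshes with random custom data and some raised, or numbered child actors with optional random height, biome and water/land values.
; An optional WaveFunctionCollapse pass starts at a chosen child tile and sweeps the list, using capsule overlaps to update uncompleted neighbors.
; Despite its name, that pass assigns one fixed hex type with increasing height, without constraint solving.
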(event EventBeginPlay)

(event Collision|EventActorBeginOverlap
  (params (OtherActor :type Actor%20Object%20Reference)))

(event EventTick
  (params (DeltaSeconds :type Float%20%28single-precision%29)))

(fn ConstructionScript
  (bind _returnvalue (Math|Random|RandomFloat))
  (bind _instancedstaticmesh (Variables|Default|GetInstancedStaticMesh))
  (Rendering|Material|SetScalarParameterValue 0 "WaterFreq" (Variables|MapSettings|GetWaterFreg) :!class /Script/Engine.KismetMaterialLibrary)
  (Variables|Default|SetScale (/ (* (Variables|GridSettings|GetHexRadius) 2.0) 173.0))
  (for _index (range 0 (Variables|GridSettings|GetHeight))
    (for _index_2 (range 0 (Variables|GridSettings|GetWidth))
      (if (Variables|GridSettings|GetInstanced?)
        (bind _returnvalue_2 (Components|InstancedStaticMesh|AddInstance (Variables|Default|GetInstancedStaticMesh) (Math|Transform|MakeTransform (Math|Vector|MakeVector (+ (* _index_2 (Variables|GridSettings|GetHexRadius) 2.0) (Variables|Default|GetOffset)) (* _index (/ (* (Variables|GridSettings|GetHexRadius) 2.0) (Math|Float|Sqrt 3.0)) 1.5) 0.0) "0, 0, 0" (Math|Conversions|ToVector(Float) (Variables|Default|GetScale))) false))
        (LocalVariables|SetInstanceIndex _returnvalue_2)
        (LocalVariables|SetLandTypeNumber _returnvalue)
        (Components|InstancedStaticMesh|SetCustomDataValue (Variables|Default|GetInstancedStaticMesh) (LocalVariables|GetInstanceIndex) 0 _returnvalue true)
        (if (>= (LocalVariables|GetLandTypeNumber) 0.6)
          (Components|InstancedStaticMesh|UpdateInstanceTransform _instancedstaticmesh (LocalVariables|GetInstanceIndex) (Math|Transform|MakeTransform (+ (.location (.OutInstanceTransform (Components|InstancedStaticMesh|GetInstanceTransform _instancedstaticmesh (LocalVariables|GetInstanceIndex) false))) "0,0,30.000000") (.rotation (.OutInstanceTransform (Components|InstancedStaticMesh|GetInstanceTransform _instancedstaticmesh (LocalVariables|GetInstanceIndex) false))) (.scale (.OutInstanceTransform (Components|InstancedStaticMesh|GetInstanceTransform _instancedstaticmesh (LocalVariables|GetInstanceIndex) false)))) false true true))
        (else
          (bind _returnvalue_3 (AddComponent|AddChildActorComponent false (Math|Transform|MakeTransform (Math|Vector|MakeVector (+ (* _index_2 (Variables|GridSettings|GetHexRadius) 2.0) (Variables|Default|GetOffset)) (* _index (/ (* (Variables|GridSettings|GetHexRadius) 2.0) (Math|Float|Sqrt 3.0)) 1.5) 0.0) "0, 0, 0" (Math|Conversions|ToVector(Float) (Variables|Default|GetScale)))))
          (Variables|Default|SetTileNumber (+ (Variables|Default|GetTileNumber) 1))
          (Utilities|Array|Add (Variables|Default|GetHexTiles) _returnvalue_3)
          (ChildActorComponent|SetChildActorClass _returnvalue_3 0)
          (bind _asbp_hex_tile (Utilities|Casting|CastTo (Variables|/Script/Engine.ChildActorComponent|GetChildActor _returnvalue_3)))
          (Rendering|Components|TextRender|SetText (Variables|Default|GetTextRender _asbp_hex_tile) (Utilities|Text|ToText(Integer) (Variables|Default|GetTileNumber)))
          (Rendering|SetBoundsScale (Variables|Default|GetHexTile _asbp_hex_tile) 2.0)
          (if (Variables|GridSettings|GetPreGenerate?)
            (CallFunction|UpdateHex _asbp_hex_tile (Math|Random|RandomFloatinRange (Variables|MapSettings|GetMinimumLandHeight) (Variables|MapSettings|GetMaximumLandHeight)) (Math|Random|RandomFloatinRange 0.0 1.0) (Math|Random|RandomFloatinRange 0.0 1.0))))))
    (Utilities|FlowControl|FlipFlop
      (:A
        (Variables|Default|SetOffset (* (Variables|GridSettings|GetHexRadius) -1.0)))
      (:B
        (Variables|Default|SetOffset 0.0))))
  (if (Variables|GridSettings|GetWaveFunctionGenerate?)
    (CallFunction|WaveFunctionCollapse (Utilities|Array|Get(acopy) (Variables|Default|GetHexTiles) (+ (Variables|MapSettings|GetStartingHexTileGen) -1)))))

(fn WaveFunctionCollapse
  (params (StartingHexTile :type Child%20Actor%20Component%20Object%20Reference))
  (LocalVariables|SetCurrentTile (Variables|MapSettings|GetStartingHexTileGen))
  (bind _asbp_hex_tile (Utilities|Casting|CastTo (Variables|/Script/Engine.ChildActorComponent|GetChildActor StartingHexTile)))
  (Utilities|Array|Add (.CompletedTiles (LocalVariables|GetCompletedTiles)) _asbp_hex_tile)
  (CallFunction|UpdateHex _asbp_hex_tile (LocalVariables|GetHeightAdjust) 0.0 0.0 0)
  (bind _outactors (Collision|CapsuleOverlapActors (Transformation|GetActorLocation _asbp_hex_tile) 2e+02 2e+02 (Utilities|Array|MakeArray "ObjectTypeQuery2") 0 (.CompletedTiles (LocalVariables|GetCompletedTiles))))
  (for _array_element _outactors
    (bind _asbp_hex_tile_2 (Utilities|Casting|CastTo _array_element))
    (Utilities|Array|Add (.CompletedTiles (LocalVariables|GetCompletedTiles)) _asbp_hex_tile_2)
    (CallFunction|UpdateHex _asbp_hex_tile_2 (+ (LocalVariables|GetHeightAdjust) 1.0) 1.0 1.0 0))
  (while (< (Utilities|Array|Length (.CompletedTiles (LocalVariables|GetCompletedTiles))) (* (+ (Variables|GridSettings|GetWidth) 1) (+ (Variables|GridSettings|GetHeight) 1)))
    (if (>= (LocalVariables|GetCurrentTile) (Utilities|Array|Length (Variables|Default|GetHexTiles)))
      (LocalVariables|SetCurrentTile 1)
      (else
        (LocalVariables|SetCurrentTile (+ 0 1 (LocalVariables|GetCurrentTile)))))
    (bind _asbp_hex_tile_3 (Utilities|Casting|CastTo (Variables|/Script/Engine.ChildActorComponent|GetChildActor (Utilities|Array|Get(acopy) (Variables|Default|GetHexTiles) (+ (LocalVariables|GetCurrentTile) -1)))))
    (bind _outactors_2 (Collision|CapsuleOverlapActors (Transformation|GetActorLocation _asbp_hex_tile_3) 2e+02 2e+02 (Utilities|Array|MakeArray "ObjectTypeQuery2") 0 (.CompletedTiles (LocalVariables|GetCompletedTiles))))
    (for _array_element_2 _outactors_2
      (bind _asbp_hex_tile_4 (Utilities|Casting|CastTo _array_element_2))
      (Utilities|Array|Add (.CompletedTiles (LocalVariables|GetCompletedTiles)) _asbp_hex_tile_4)
      (bind _output_get (LocalVariables|SetHeightAdjust (+ (LocalVariables|GetHeightAdjust) 1.0)))
      (CallFunction|UpdateHex _asbp_hex_tile_4 _output_get 1.0 1.0 0))))