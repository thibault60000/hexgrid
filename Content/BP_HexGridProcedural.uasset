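; Procedural hex terrain actor that builds a Width by Height grid of instanced tiles in its construction script, when Instanced is set.
; Tiles are spaced by mesh radius, with alternate rows shifted.
; Two FastNoise layers sampled at world position set each tile's height, with optional flat water and a depth multiplier below zero.
; Height also feeds per-instance custom data, the water threshold feeds MPC_HexGrid, and a water plane scales to the grid.
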(event EventBeginPlay)

(event Collision|EventActorBeginOverlap
  (params (OtherActor :type Actor%20Object%20Reference)))

(event EventTick
  (params (DeltaSeconds :type Float%20%28single-precision%29)))

(fn ConstructionScript
  (bind _noiselevel1 (Variables|Default|GetNoiseLevel1))
  (bind _noiselevel2 (Variables|Default|GetNoiseLevel2))
  ;[0.1232 0.3635 1] Fast Noise Level 1
  (bind _returnvalue (Game|ConstructObjectfromClass "/Script/FastNoiseGenerator.FastNoiseWrapper"))
  (bind _output_get (Variables|FastNoise1|SetNoiseWrapperLevel1 _returnvalue))
  (Class|FastNoiseWrapper|SetupFastNoise _output_get (Variables|FastNoise1|GetNoise%20Type1) (Variables|FastNoise1|GetSeed1) (Variables|FastNoise1|GetFrequency1) (Variables|FastNoise1|GetInterp1) (Variables|FastNoise1|GetFractaltype1) (Variables|FastNoise1|GetOctaves1) (Variables|FastNoise1|GetLacunarity1) (Variables|FastNoise1|GetGain1) (Variables|FastNoise1|GetCellular%20Jitter1) (Variables|FastNoise1|GetCellularDistance1) (Variables|FastNoise1|GetCellularReturn1))
  ;[1 0.4417 0.7828] Fast Noise level 2
  (bind _returnvalue_2 (Game|ConstructObjectfromClass "/Script/FastNoiseGenerator.FastNoiseWrapper"))
  (bind _output_get_2 (Variables|FastNoise2|SetNoise%20Wrapper%20Level%202 _returnvalue_2))
  (Class|FastNoiseWrapper|SetupFastNoise _output_get_2 (Variables|FastNoise2|GetNoise%20Type%202) (Variables|FastNoise2|GetSeed%202) (Variables|FastNoise2|GetFrequency%202) (Variables|FastNoise2|GetInterp%202) (Variables|FastNoise2|GetFractaltype%202) (Variables|FastNoise2|GetOctaves%202) (Variables|FastNoise2|GetLacunarity%202) (Variables|FastNoise2|GetGain%202) (Variables|FastNoise2|GetCellular%20Jitter%202) (Variables|FastNoise2|GetCellularDistance%202) (Variables|FastNoise2|GetCellularReturn%202))
  ;[0.5255 1 0.5061] Get static Mesh radius
  (Components|StaticMesh|SetStaticMesh (Variables|Default|GetInstancedStaticMesh) (Variables|GridOptions|GetTileMesh))
  (Variables|GridOptions|SetRadius (* (.x (.max (StaticMesh|GetBoundingBox (Variables|GridOptions|GetTileMesh)))) (Variables|GridOptions|GetScale)))
  ;[0.9247 1 0.1517] Height Loop
  (for _index (range 0 (- (Variables|GridOptions|GetHeight) 1))
    ;[1 0.5036 0.1971] Width Loop
    (for _index_2 (range 0 (- (Variables|GridOptions|GetWidth) 1))
      (if (Variables|GridOptions|GetInstanced?)
        ;[1 0.1968 0.2366] Instanced Mesh
        (bind _returnvalue_3 (Components|InstancedStaticMesh|AddInstance (Variables|Default|GetInstancedStaticMesh) (Math|Transform|MakeTransform (Math|Vector|MakeVector (+ (* _index_2 (Variables|GridOptions|GetRadius) 2.0) (* _index_2 (Variables|GridOptions|GetOffset)) (Variables|GridOptions|GetRowOffset)) (+ (* (/ (* (Variables|GridOptions|GetRadius) 2.0) (Math|Float|Sqrt 3.0)) 1.5 _index) (* _index (Variables|GridOptions|GetOffset))) 0.0) "0, 0, 0" (Math|Conversions|ToVector(Float) (Variables|GridOptions|GetScale))) false))
        (Rendering|Material|SetScalarParameterValue "/Game/MPC_HexGrid.MPC_HexGrid" "WaterThreshold" (Variables|GridOptions|GetWaterThresold) :!class /Script/Engine.KismetMaterialLibrary)
        ;[1 0.9013 0.5207] Transform (random) Instancied Mesh (tile height)
        (Variables|instancedtileoptions|SetTileInstanceIndex _returnvalue_3)
        (if (and (<= (Class|FastNoiseWrapper|GetNoise2D (Variables|FastNoise1|GetNoiseWrapperLevel1) (* (.x (.location (.OutInstanceTransform (Components|InstancedStaticMesh|GetInstanceTransform (Variables|Default|GetInstancedStaticMesh) (Variables|instancedtileoptions|GetTileInstanceIndex) true)))) _noiselevel1) (* (.y (.location (.OutInstanceTransform (Components|InstancedStaticMesh|GetInstanceTransform (Variables|Default|GetInstancedStaticMesh) (Variables|instancedtileoptions|GetTileInstanceIndex) true)))) _noiselevel1)) (Variables|GridOptions|GetWaterThresold)) (Variables|InstancedTileOptions|GetFlatWaterTile))
          ;[0.365 0.566 1] Flat Water Tile Settings
          (Variables|InstancedTileOptions|SetTileHeight (+ (Variables|GridOptions|GetWaterThresold) (Variables|GridOptions|GetBaseWaterHeight)))
          (elif (< (+ (Class|FastNoiseWrapper|GetNoise2D (Variables|FastNoise1|GetNoiseWrapperLevel1) (* (.x (.location (.OutInstanceTransform (Components|InstancedStaticMesh|GetInstanceTransform (Variables|Default|GetInstancedStaticMesh) (Variables|instancedtileoptions|GetTileInstanceIndex) true)))) _noiselevel1) (* (.y (.location (.OutInstanceTransform (Components|InstancedStaticMesh|GetInstanceTransform (Variables|Default|GetInstancedStaticMesh) (Variables|instancedtileoptions|GetTileInstanceIndex) true)))) _noiselevel1)) (Math|Float|Clamp(Float) (Class|FastNoiseWrapper|GetNoise2D (Variables|FastNoise2|GetNoise%20Wrapper%20Level%202) (* (.x (.location (.OutInstanceTransform (Components|InstancedStaticMesh|GetInstanceTransform (Variables|Default|GetInstancedStaticMesh) (Variables|instancedtileoptions|GetTileInstanceIndex) true)))) _noiselevel2) (* (.y (.location (.OutInstanceTransform (Components|InstancedStaticMesh|GetInstanceTransform (Variables|Default|GetInstancedStaticMesh) (Variables|instancedtileoptions|GetTileInstanceIndex) true)))) _noiselevel2)) -1.0) 0.0) 0.0)
            (Variables|InstancedTileOptions|SetTileHeight (* (Variables|GridOptions|GetWaterDepthMultiplier) (+ (Class|FastNoiseWrapper|GetNoise2D (Variables|FastNoise1|GetNoiseWrapperLevel1) (* (.x (.location (.OutInstanceTransform (Components|InstancedStaticMesh|GetInstanceTransform (Variables|Default|GetInstancedStaticMesh) (Variables|instancedtileoptions|GetTileInstanceIndex) true)))) _noiselevel1) (* (.y (.location (.OutInstanceTransform (Components|InstancedStaticMesh|GetInstanceTransform (Variables|Default|GetInstancedStaticMesh) (Variables|instancedtileoptions|GetTileInstanceIndex) true)))) _noiselevel1)) (Math|Float|Clamp(Float) (Class|FastNoiseWrapper|GetNoise2D (Variables|FastNoise2|GetNoise%20Wrapper%20Level%202) (* (.x (.location (.OutInstanceTransform (Components|InstancedStaticMesh|GetInstanceTransform (Variables|Default|GetInstancedStaticMesh) (Variables|instancedtileoptions|GetTileInstanceIndex) true)))) _noiselevel2) (* (.y (.location (.OutInstanceTransform (Components|InstancedStaticMesh|GetInstanceTransform (Variables|Default|GetInstancedStaticMesh) (Variables|instancedtileoptions|GetTileInstanceIndex) true)))) _noiselevel2)) -1.0) 0.0)))
            (else
              (Variables|InstancedTileOptions|SetTileHeight (+ (Class|FastNoiseWrapper|GetNoise2D (Variables|FastNoise1|GetNoiseWrapperLevel1) (* (.x (.location (.OutInstanceTransform (Components|InstancedStaticMesh|GetInstanceTransform (Variables|Default|GetInstancedStaticMesh) (Variables|instancedtileoptions|GetTileInstanceIndex) true)))) _noiselevel1) (* (.y (.location (.OutInstanceTransform (Components|InstancedStaticMesh|GetInstanceTransform (Variables|Default|GetInstancedStaticMesh) (Variables|instancedtileoptions|GetTileInstanceIndex) true)))) _noiselevel1)) (Math|Float|Clamp(Float) (Class|FastNoiseWrapper|GetNoise2D (Variables|FastNoise2|GetNoise%20Wrapper%20Level%202) (* (.x (.location (.OutInstanceTransform (Components|InstancedStaticMesh|GetInstanceTransform (Variables|Default|GetInstancedStaticMesh) (Variables|instancedtileoptions|GetTileInstanceIndex) true)))) _noiselevel2) (* (.y (.location (.OutInstanceTransform (Components|InstancedStaticMesh|GetInstanceTransform (Variables|Default|GetInstancedStaticMesh) (Variables|instancedtileoptions|GetTileInstanceIndex) true)))) _noiselevel2)) -1.0) 0.0)))))
        (Components|InstancedStaticMesh|UpdateInstanceTransform (Variables|Default|GetInstancedStaticMesh) (Variables|instancedtileoptions|GetTileInstanceIndex) (Math|Transform|MakeTransform (+ (.location (.OutInstanceTransform (Components|InstancedStaticMesh|GetInstanceTransform (Variables|Default|GetInstancedStaticMesh) (Variables|instancedtileoptions|GetTileInstanceIndex) true))) (Math|Vector|MakeVector 0.0 0.0 (+ (* (+ (Variables|InstancedTileOptions|GetTileHeight) 0.0) (Variables|GridOptions|GetTileHeightStrenght)) (Variables|InstancedTileOptions|GetTileHeightOffset)))) "0, 0, 0" (Math|Conversions|ToVector(Float) (Variables|GridOptions|GetScale))) true false false)
        ;[0.4515 1 0.2033] Set Tile Height with CustomData on Material
        (Components|InstancedStaticMesh|SetCustomDataValue (Variables|Default|GetInstancedStaticMesh) (Variables|instancedtileoptions|GetTileInstanceIndex) 0 (Variables|InstancedTileOptions|GetTileHeight) true)))
    ;[1 0.3571 0.8886] Gestion du décalage une ligne de Tile sur 2
    (Utilities|FlowControl|FlipFlop
      (:A
        (Variables|GridOptions|SetRowOffset (* (Variables|GridOptions|GetRadius) -1.0)))
      (:B
        (Variables|GridOptions|SetRowOffset 0.0))))
  ;[0.0831 1 0.9801] Génération du Plane pour l'eau
  (Transformation|SetWorldScale3D (Variables|Default|GetStaticMesh) (Math|Vector|MakeVector (Math|Conversions|ToFloat(Integer) (Variables|GridOptions|GetWidth)) (* (Math|Conversions|ToFloat(Integer) (Variables|GridOptions|GetHeight)) 0.75) 1.0)))